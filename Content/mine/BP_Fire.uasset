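; BP_Fire is a fire light-source actor whose particle effect fades in and out with the day/night state.
; BeginPlay adds an audio component and sets the particle system to full scale.
; Each Tick steps the uniform particle scale by a fixed amount within zero and its maximum, shrinking while IsNight is true and growing otherwise.
; The flag reads inverted: the comments label the shrinking branch morning and the growing branch night.
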(event `self.ReceiveBeginPlay`
  (`AddComponent|NODE_AddAudioComponent-0`)
  (set `self.particle_max` 3.0)
  (bind _output_get (set `self.particle` 3.0))
  (`SceneComponent.SetWorldScale3D` (`self.ParticleSystem`) (`KismetMathLibrary.MakeVector` _output_get _output_get _output_get)))

(event `self.ReceiveTick`
  (params (DeltaSeconds :type "Float (single-precision)"))
  (bind _particle (`self.particle`))
  (bind _particle_2 (`self.particle`))
  (if (`self.is_night`)
    ;[1 1 1] 朝だとして光源を消す
    (bind _output_get (set `self.particle` (- (`self.particle`) 0.05)))
    (if (>= _output_get 0.0)
      (`SceneComponent.SetWorldScale3D` (`self.ParticleSystem`) (`KismetMathLibrary.MakeVector` _particle_2 _particle_2 _particle_2))
      (else
        (set `self.particle` 0.0)))
    (else
      ;[1 1 1] 夜だとして光源を出す
      (bind _output_get_2 (set `self.particle` (+ (`self.particle`) 0.05)))
      (if (>= _output_get_2 (`self.particle_max`))
        (set `self.particle` (`self.particle_max`))
        (else
          (`SceneComponent.SetWorldScale3D` (`self.ParticleSystem`) (`KismetMathLibrary.MakeVector` _particle _particle _particle)))))))

(fn `UserConstructionScript`)