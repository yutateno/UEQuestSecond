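; BP_PointLight is a point light actor that fades on at night and off by day, driven by an IsNight flag.
; BeginPlay starts it as daytime with zero intensity and sets a maximum brightness.
; Each Tick steps the intensity up or down by a fixed, frame-based amount, clamps it at the limits, and applies it to the PointLight while within range.
; Nothing in this Blueprint switches IsNight after initialization.
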(event `self.ReceiveBeginPlay`
  (set `self.is_night` false)
  (set `self.light_intensity` 0.0)
  (set `self.light_intensity_max` 1500.0))

(event `self.ReceiveTick`
  (params (DeltaSeconds :type "Float (single-precision)"))
  (if (`self.is_night`)
    ;[1 1 1] 夜だとして光源を出す
    (bind _output_get (set `self.light_intensity` (+ (`self.light_intensity`) 5.0)))
    (if (>= _output_get (`self.light_intensity_max`))
      (set `self.light_intensity` 1500.0)
      (else
        (`LightComponent.SetIntensity` (`self.PointLight`) (`self.light_intensity`))))
    (else
      ;[1 1 1] 朝だとして光源を消す
      (bind _output_get_2 (set `self.light_intensity` (- (`self.light_intensity`) 5.0)))
      (if (>= _output_get_2 0.0)
        (`LightComponent.SetIntensity` (`self.PointLight`) (`self.light_intensity`))
        (else
          (set `self.light_intensity` 0.0))))))

(fn `UserConstructionScript`)